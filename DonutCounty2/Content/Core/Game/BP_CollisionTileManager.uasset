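; Manager actor that fills a grid with BP_CollisionTile actors, presumably to provide tiled collision for the game.
; On BeginPlay or RegenerateGrid, ForEachTilePosition invokes a callback that spawns a scaled tile and appends it to Tiles.
; RegenerateGrid does not clear existing tiles in this graph.
; A leftover procedural mesh attempt builds quads through AddTile, but its collision-enabled mesh creation call is disconnected.
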(event `CustomEvent`
  (params (Location :type "Vector Structure") (Scale :type "Float (single-precision)"))
  ; Attempt with procedural mesh
  (`self.AddTile` Location (`self.Vertices`) (`self.Triangles`)))

(event `self.ReceiveBeginPlay`
  (`self.ForEachTilePosition` (delegate `DoForTilePosition`) :!label _label))

(event `RegenerateGrid`
  (goto _label))

(event `DoForTilePosition`
  (params (Location :type "Vector Structure") (Scale :type "Float (single-precision)"))
  (bind _returnvalue (`|SpawnActorFromClass` "/Game/Core/Game/BP_CollisionTile.BP_CollisionTile_C" (`KismetMathLibrary.MakeTransform` Location (struct) (`KismetMathLibrary.Conv_DoubleToVector` Scale)) "Undefined" "MultiplyWithRoot" null null))
  (`KismetArrayLibrary.Array_Add` (`self.Tiles`) _returnvalue))

(fn `UserConstructionScript`)