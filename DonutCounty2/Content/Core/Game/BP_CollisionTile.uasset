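; Tile actor meant to show player overlap by switching its Plane material to red while the player pawn is inside and green after it leaves.
; Custom overlap events filter for player pawn 0 and set the material.
; The setup chain that creates both dynamic materials from engine vertex-color view materials, binds those events and applies the initial color has no entry event, so it never runs.
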(event `OnActorEndOverlap_Event` :!signature `self.OnActorEndOverlap`
  (params (OverlappedActor :type "Actor Object Reference") (OtherActor :type "Actor Object Reference"))
  (if (== OtherActor (`GameplayStatics.GetPlayerPawn` 0))
    (`PrimitiveComponent.SetMaterial` (`self.Plane`) 0 (`self.MatGreen`))))

(event `OnActorBeginOverlap_Event` :!signature `self.OnActorBeginOverlap`
  (params (OverlappedActor :type "Actor Object Reference") (OtherActor :type "Actor Object Reference"))
  (if (== OtherActor (`GameplayStatics.GetPlayerPawn` 0))
    (`PrimitiveComponent.SetMaterial` (`self.Plane`) 0 (`self.MatRed`))))

(fn `UserConstructionScript`)