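; BP_DynamicMesh is a Blueprint that builds a flat square tile at runtime on a procedural mesh, with collision.
; AddTile appends four corners, sized by Resolution, and two triangles' indices to the Vertices and Triangles arrays, which then feed CreateMeshSectionLinearColor.
; BeginPlay and the AddMesh event share this path, always using the same raised origin, so repeat calls append overlapping geometry.
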(event `self.ReceiveBeginPlay`
  (`self.AddTile` (0.0 0.0 100.0) (`self.Vertices`) (`self.Triangles`) :!label _label)
  (`ProceduralMeshComponent.CreateMeshSection_LinearColor` :`self` (`self.ProceduralMesh`) :`Vertices` (`self.Vertices`) :`Triangles` (`self.Triangles`) :`bCreateCollision` true))

(event `AddMesh`
  (goto _label))

(fn `UserConstructionScript`)