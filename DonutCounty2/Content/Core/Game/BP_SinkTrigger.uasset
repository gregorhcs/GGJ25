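; BP_SinkTrigger is a trigger actor that modifies the player sink's radius and plays a devour sound when its box is overlapped.
; One tick after BeginPlay it finds and caches the CollisionTileManager and BP_PlayerSink actors.
; Every overlap, with no filter on the other actor, passes the same fixed value to both radius functions, then plays the sound quietly at the sink's location.
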(event `self.ReceiveBeginPlay`
  (`KismetSystemLibrary.DelayUntilNextTick`)
  (bind _returnvalue (`GameplayStatics.GetActorOfClass` "/Script/DonutCounty2.CollisionTileManager"))
  (set `self.CollisionTileManager` _returnvalue)
  (bind _returnvalue_2 (`GameplayStatics.GetActorOfClass` "/Game/Core/Player/BP_PlayerSink.BP_PlayerSink_C"))
  (set `self.PlayerSink` _returnvalue_2))

(event `self.Box.OnComponentBeginOverlap`
  (params (OverlappedComponent :type "PrimitiveComponent Object Reference") (OtherActor :type "Actor Object Reference") (OtherComp :type "PrimitiveComponent Object Reference") (OtherBodyIndex :type Integer) (bFromSweep :type Boolean) (SweepResult :type "HitResult Structure (by ref)"))
  (`CollisionTileManager.ModifySinkRadiusInTiles` (`self.CollisionTileManager`) 1.04)
  (`/Game/Core/Player/BP_PlayerSink.ModifySinkRadius` (`self.PlayerSink`) 1.04)
  (`GameplayStatics.PlaySoundAtLocation` "/Game/Core/Player/MS_Devour.MS_Devour" (`self.K2_GetActorLocation` (`self.PlayerSink`)) (struct) 0.1 1.0 0.0 null null null null))

(fn `UserConstructionScript`)